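; Player character Blueprint that serves as a keyboard-driven test bed for animation montage playback.
; Q, E and R play test montages, including a root motion variant and one that starts at a named section.
; Number keys stop either a specific montage or whichever is currently playing.
; P switches the mesh to another animation class at runtime.
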(event `Key|R`
  (params (Key :type "Key Structure"))
  ;[1 1 1] Montage Test
  (:`Pressed`
    (`self.PlayAnimMontage` "/Game/AnimationSystem/Animations/Montage/Montage_RootMotion_TestA.Montage_RootMotion_TestA")))

(event `Key|One`
  (params (Key :type "Key Structure"))
  ;[1 1 1] Montage Test
  (:`Pressed`
    (`self.StopAnimMontage` "/Game/AnimationSystem/Animations/Montage/Montage_TestA.Montage_TestA")))

(event `Key|Q`
  (params (Key :type "Key Structure"))
  ;[1 1 1] Montage Test
  (:`Pressed`
    (`self.PlayAnimMontage` "/Game/AnimationSystem/Animations/Montage/Montage_TestA.Montage_TestA")))

(event `Key|Two`
  (params (Key :type "Key Structure"))
  ;[1 1 1] Montage Test
  (:`Pressed`
    (`self.StopAnimMontage` (`self.GetCurrentMontage`))))

(event `Key|E`
  (params (Key :type "Key Structure"))
  ;[1 1 1] Montage Test
  (:`Pressed`
    (`self.PlayAnimMontage` "/Game/AnimationSystem/Animations/Montage/Montage_TestB.Montage_TestB" 1.0 "Section1")))

(event `Key|Three`
  (params (Key :type "Key Structure"))
  ;[1 1 1] Montage Test
  (:`Pressed`
    (`self.StopAnimMontage` "/Game/AnimationSystem/Animations/Montage/Montage_TestB.Montage_TestB")))

(event `Key|P`
  (params (Key :type "Key Structure"))
  (:`Pressed`
    (`SkeletalMeshComponent.SetAnimInstanceClass` (`self.Mesh`) "/Game/AnimationSystem/AnimPose_1.AnimPose_1_C")))

(event `self.ReceiveBeginPlay`)

(fn `UserConstructionScript`)