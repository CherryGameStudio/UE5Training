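; BP_MyCharacter is a character Blueprint with Gameplay Ability System attack and block abilities and a widget-component nameplate.
; Keys 1 and 2 activate the Ability.Attack and Ability.Block abilities by tag, with remote activation allowed.
; BeginPlay binds the character to its Widget_CharacterPate, and attribute set updates pass through a client update event to refresh that widget.
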(event `self.ReceiveBeginPlay`
  (bind _aswidget_character_pate (cast `/Game/Blueprints/Widget_CharacterPate` (`WidgetComponent.GetWidget` (`self.WidgetComponent`))))
  (`/Game/Blueprints/Widget_CharacterPate.SetCharacterParams` _aswidget_character_pate self))

(event `Key|One`
  (params (Key :type "Key Structure"))
  (:`Pressed`
    (`AbilitySystemComponent.TryActivateAbilitiesByTag` (`self.GetAbilitySystemComponent`) (`BlueprintGameplayTagLibrary.MakeGameplayTagContainerFromTag` (struct :`TagName` "Ability.Attack")) true)))

(event `Key|Two`
  (params (Key :type "Key Structure"))
  (:`Pressed`
    (`AbilitySystemComponent.TryActivateAbilitiesByTag` (`self.GetAbilitySystemComponent`) (`BlueprintGameplayTagLibrary.MakeGameplayTagContainerFromTag` (struct :`TagName` "Ability.Block")) true)))

(event `self.OnAttributeSetUpdate`
  (`self.Client_Update`))

(event `Client_Update`
  (`self.Client_UpdateUI`))

(fn `Client_UpdateUI`
  (bind _aswidget_character_pate (cast `/Game/Blueprints/Widget_CharacterPate` (`WidgetComponent.GetWidget` (`self.WidgetComponent`))))
  (`/Game/Blueprints/Widget_CharacterPate.UpdateCharacterParams` _aswidget_character_pate))

(fn `UserConstructionScript`)