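; Blueprint function library with a FindTarget helper that finds a Character in front of a source actor.
; It sweeps an oriented box forward along the actor's facing against Pawn objects, ignores the source, and draws debug shapes.
; The hit actor is cast to Character, and a failed cast returns empty so a stale result from a previous call is not reused.
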(fn `FindTarget`
  (params (Source :type "Character Object Reference"))
  (returns (Target :type "Character Object Reference"))
  (bind _returnvalue (`Actor.GetActorForwardVector` Source))
  (bind _returnvalue_2 (`Actor.K2_GetActorLocation` Source))
  (bind _outhit (`KismetSystemLibrary.BoxTraceSingleForObjects` Source _returnvalue_2 (+ _returnvalue_2 (* _returnvalue 1000.0)) (0.0 50.0 90.0) (`KismetMathLibrary.Conv_VectorToRotator` _returnvalue) (`|MakeArray` (enumliteral `EObjectTypeQuery` "ObjectTypeQuery3")) false (`|MakeArray` Source :!type "Actor Object Reference") "ForDuration" true (struct :`R` 1.0 :`A` 1.0) (struct :`G` 1.0 :`A` 1.0) 2.0))
  ;[1 1 1] 这里Cast Failed的时候必须清理一下缓存，避免拿到上一次的结果。
  (bind _ascharacter (cast `Character` (`.HitActor` (`GameplayStatics.BreakHitResult` _outhit)))
    (:`then`
      (return _ascharacter))
    (:`CastFailed`
      (return null))))